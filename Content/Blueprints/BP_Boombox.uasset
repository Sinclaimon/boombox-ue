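; BP_Boombox is an interactive boombox that the player can switch on and off while standing inside its interaction radius.
; Overlap events track the third-person character, and the Enhanced Input interact action toggles the display material and song when the player is in range.
; While on, the BoomboxAnim timeline's Intensity track scales both speakers.
; Switching off stops the timeline and restores the scale cached from Speaker1 at BeginPlay.
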(event `self.ReceiveBeginPlay`
  (`EnhancedInputSubsystemInterface.AddMappingContext` (pcsubsystem `EnhancedInputLocalPlayerSubsystem` (`GameplayStatics.GetPlayerController` 0)) "/Game/ThirdPerson/Input/IMC_Boombox.IMC_Boombox" 0 (struct))
  (set `self.InitialSpeakerScale` (`SceneComponent.K2_GetComponentScale` (`self.Speaker1`))))

(event `self.InteractionRadius.OnComponentBeginOverlap`
  (params (OverlappedComponent :type "PrimitiveComponent Object Reference") (OtherActor :type "Actor Object Reference") (OtherComp :type "PrimitiveComponent Object Reference") (OtherBodyIndex :type Integer) (bFromSweep :type Boolean) (SweepResult :type "HitResult Structure (by ref)"))
  ;[1 1 1] Interaction radius overlap handling for the player
  (cast `/Game/ThirdPerson/Blueprints/BP_ThirdPersonCharacter` OtherActor)
  (`KismetSystemLibrary.PrintString` "Actor overlapping")
  (set `self.PlayerInRadius` true))

(event `self.InteractionRadius.OnComponentEndOverlap`
  (params (OverlappedComponent :type "PrimitiveComponent Object Reference") (OtherActor :type "Actor Object Reference") (OtherComp :type "PrimitiveComponent Object Reference") (OtherBodyIndex :type Integer))
  ;[1 1 1] Interaction radius overlap handling for the player
  (cast `/Game/ThirdPerson/Blueprints/BP_ThirdPersonCharacter` OtherActor)
  (set `self.PlayerInRadius` false))

(event `EnhancedInput|/Game/ThirdPerson/Input/Actions/IA_Interact`
  (params (ActionValue :type Boolean) (ElapsedSeconds :type "Float (double-precision)") (TriggeredSeconds :type "Float (double-precision)") (InputAction :type "InputAction Object Reference" :default "/Game/ThirdPerson/Input/Actions/IA_Interact.IA_Interact"))
  ;[1 1 1] Input action for turning the boombox on/off
  (:`Started`
    (if (`self.PlayerInRadius`)
      (`self.OnOffSwitch`)
      (if (`self.TurnedOn`)
        ;[1 1 1] Speaker animation
        (bind (_direction _intensity) (`Timeline|BoomboxAnim` :!label _label)
          (:`Update`
            (bind _returnvalue (/ _intensity (`self.IntensityScaling`)))
            (`SceneComponent.SetWorldScale3D` (`self.Speaker1`) (`KismetMathLibrary.Conv_DoubleToVector` _returnvalue))
            (`SceneComponent.SetWorldScale3D` (`self.Speaker2`) (`KismetMathLibrary.Conv_DoubleToVector` _returnvalue))))
        (else
          (`self.ResetSpeakerScale`)
          (goto _label :!via `Stop`))))))

(fn `OnOffSwitch`
  ;[1 1 1] Flip the switch
  (set `self.TurnedOn` (not (`self.TurnedOn`)))
  (if (`self.TurnedOn`)
    ;[1 1 1] Turning the boombox on
    (`KismetSystemLibrary.PrintString` "Boombox on")
    (`PrimitiveComponent.SetMaterial` (`self.Display`) 0 "/Game/StarterContent/Materials/M_DisplayOn.M_DisplayOn")
    (`ActorComponent.Activate` (`self.Song`) false)
    (else
      ;[1 1 1] Turning the boombox off
      (`KismetSystemLibrary.PrintString` "Boombox off")
      (`PrimitiveComponent.SetMaterial` (`self.Display`) 0 "/Game/StarterContent/Materials/M_DisplayOff.M_DisplayOff")
      (`ActorComponent.Deactivate` (`self.Song`)))))

(fn `UserConstructionScript`)